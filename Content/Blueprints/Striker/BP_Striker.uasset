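; BP_Striker is a kick-based melee combat character that builds on its parent Blueprint's skill and movement systems.
; BeginPlay sets its base and combat blendspaces, then registers attack montages in three skill types of increasing range, some with super armour.
; Each Tick, while alive and attacking, it snaps its yaw toward a valid target, except during the aerial kick montage.
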(event EventBeginPlay
  (|CallParentFunction)
  (CallFunction|SetBaseBS "/Game/Animations/BlendSpace/Blade/BS_BladeBaseMasterMovement.BS_BladeBaseMasterMovement")
  (CallFunction|SetCombatBS "/Game/Animations/BlendSpace/Striker/BS_StrikerCombatMovement.BS_StrikerCombatMovement")
  (Utilities|FlowControl|Sequence
    (:then_0
      (CallFunction|AddSkill "NewEnumerator0" "/Game/Animations/Montage/Striker/AM_kick_01.AM_kick_01" 1.5e+02 false)
      (CallFunction|AddSkill "NewEnumerator0" "/Game/Animations/Montage/Striker/AM_kick_02.AM_kick_02" 1.5e+02 false)
      (CallFunction|AddSkill "NewEnumerator0" "/Game/Animations/Montage/Striker/AM_kick_03.AM_kick_03" 1.5e+02 false)
      (CallFunction|AddSkill "NewEnumerator0" "/Game/Animations/Montage/Striker/AM_kick_05.AM_kick_05" 1.5e+02 false)
      (CallFunction|AddSkill "NewEnumerator0" "/Game/Animations/Montage/Striker/AM_Versus_02.AM_Versus_02" 1.5e+02 false)
      (CallFunction|AddSkill "NewEnumerator0" "/Game/Animations/Montage/Striker/AM_Versus_01.AM_Versus_01" 1.5e+02 false)
      (CallFunction|AddSkill "NewEnumerator1" "/Game/Animations/Montage/Striker/AM_kick_04.AM_kick_04" 2.5e+02 false)
      (CallFunction|AddSkill "NewEnumerator1" "/Game/Animations/Montage/Striker/AM_kick_06.AM_kick_06" 2.5e+02 true)
      (CallFunction|AddSkill "NewEnumerator1" "/Game/Animations/Montage/Striker/AM_kick_08.AM_kick_08" 2.5e+02 false)
      (CallFunction|AddSkill "NewEnumerator2" "/Game/Animations/Montage/Striker/AM_kick_07.AM_kick_07" 5e+02 true)
      (CallFunction|AddSkill "NewEnumerator2" "/Game/Animations/Montage/Striker/AM_kick_Air.AM_kick_Air" 4e+02 true))))

(event Collision|EventActorBeginOverlap
  (params (OtherActor :type Actor%20Object%20Reference)))

(event EventTick
  (params (DeltaSeconds :type Float%20%28single-precision%29))
  (|CallParentFunction DeltaSeconds)
  (|LookAtTargetByAttacking))

(fn ConstructionScript
  (|CallParentFunction))
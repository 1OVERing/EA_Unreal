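; Base monster Character that reacts to air-juggle and shoot-down attacks, with gravity scale set from Game Instance options.
; AnyDamage casts the damage type: air attacks switch movement to Flying until a timeline ends, while shoot-downs end air mode immediately.
; During a shoot-down, Tick repeatedly launches the monster downward until near the ground.
; A downward line trace measures ground distance, choosing Falling or Walking and ending the slam, with optional debug drawing.
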(event Custom|ShootDown
  (Variables|Default|SetIsShootDown true)
  (CallFunction|AirModeEnd))

(event EventBeginPlay
  (Utilities|FlowControl|Sequence
    (:then_0
      (|Node_DefaultSetting))))

(event Collision|EventActorBeginOverlap
  (params (OtherActor :type Actor%20Object%20Reference)))

(event EventTick
  (params (DeltaSeconds :type Float%20%28single-precision%29))
  (CallFunction|UpdateShootDown))

(event Game|Damage|EventAnyDamage
  (params (Damage :type Float%20%28single-precision%29) (DamageType :type Damage%20Type%20Object%20Reference) (InstigatedBy :type Controller%20Object%20Reference) (DamageCauser :type Actor%20Object%20Reference))
  (Utilities|FlowControl|Sequence
    (:then_0
      (Utilities|Casting|CastToDTBP_AirAttack DamageType)
      (CallFunction|PlayAirMode))
    (:then_1
      (Utilities|Casting|CastToDTBP_ShootDown DamageType)
      (CallFunction|ShootDown))))

(event EventAirModeEnd
  (if (> (CallFunction|LandingCheck) 5e+01)
    (Pawn|Components|CharacterMovement|SetMovementMode (Variables|Character|GetCharacterMovement) "MOVE_Falling" 0)
    (else
      (Pawn|Components|CharacterMovement|SetMovementMode (Variables|Character|GetCharacterMovement) "MOVE_Walking" 0)))
  (Variables|Default|SetAirMode false))

(event EventPlayAirMode
  (Pawn|Components|CharacterMovement|SetMovementMode (Variables|Character|GetCharacterMovement) "MOVE_Flying" 0)
  (Variables|Default|SetAirMode true)
  (Timeline|EndAirModeTimer PlayFromStart
    (:Finished
      (CallFunction|AirModeEnd))))

(fn ConstructionScript)

(fn LandingCheck
  (bind _returnvalue (Transformation|GetActorLocation))
  (bind _capsulecomponent (Variables|Collision|GetCapsuleComponent))
  (bind _returnvalue_2 (Components|Capsule|GetScaledCapsuleHalfHeight _capsulecomponent))
  (bind _returnvalue_3 (- (.z _returnvalue) _returnvalue_2))
  (Utilities|FlowControl|Sequence
    (:then_0
      (bind _asbp_game_instance (Utilities|Casting|CastToBP_GameInstance (Game|GetGameInstance)))
      (if (.OnAttackDebugTrace (Utilities|Struct|BreakF_GameOption (Variables|/Game/Blueprints/Systems/BP_GameInstance.BP_GameInstance_C|GetGameOption _asbp_game_instance)))
        (LocalVariables|SetDrawType "ForDuration")
        (else
          (LocalVariables|SetDrawType "None"))))
    (:then_1
      (bind (_outhit _returnvalue_4) (Collision|LineTraceByChannel (Math|Vector|MakeVector (.x _returnvalue) (.y _returnvalue) _returnvalue_3) (Math|Vector|MakeVector (.x _returnvalue) (.y _returnvalue) (- _returnvalue_3 2e+03)) "TraceTypeQuery1" false 0 (LocalVariables|GetDrawType)))
      (if _returnvalue_4
        (return (.Distance (Collision|BreakHitResult _outhit)))
        (else
          (return 1e+04))))))

(fn UpdateShootDown
  (if (Variables|Default|GetIsShootDown)
    (if (> (CallFunction|LandingCheck) 1e+02)
      (Character|LaunchCharacter "0.000000,0.000000,-1000.000000" false false)
      (else
        (Variables|Default|SetIsShootDown false)))))
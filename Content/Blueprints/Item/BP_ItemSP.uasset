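; BP_ItemSP is a pickup item that gives SP to the player.
; When the player character overlaps Coll_Sphere and implements BPI_Item, it passes its SP value through the AddSPMessage interface call and destroys itself.
; The construction script gives the actor a random rotation without roll.
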(event OnComponentBeginOverlap(Coll_Sphere)
  (params (OverlappedComponent :type Primitive%20Component%20Object%20Reference) (OtherActor :type Actor%20Object%20Reference) (OtherComp :type Primitive%20Component%20Object%20Reference) (OtherBodyIndex :type Integer) (bFromSweep :type Boolean) (SweepResult :type Hit%20Result%20Structure%20%28by%20ref%29))
  (if (== OtherActor (Game|GetPlayerCharacter 0))
    (if (Utilities|DoesObjectImplementInterface OtherActor "/Game/Blueprints/Interface/BPI_Item.BPI_Item_C")
      (Class|BPIItem|AddSP(Message) OtherActor (Variables|Default|GetSP))
      (Actor|DestroyActor))))

(event EventBeginPlay)

(event Collision|EventActorBeginOverlap
  (params (OtherActor :type Actor%20Object%20Reference)))

(event EventTick
  (params (DeltaSeconds :type Float%20%28single-precision%29)))

(fn ConstructionScript
  (bind _returnvalue (Math|Random|RandomRotator false))
  (Transformation|SetActorRotation (Math|Rotator|MakeRotator (.roll _returnvalue) (.pitch _returnvalue) (.yaw _returnvalue))))
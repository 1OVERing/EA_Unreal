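; Spawns waves of Blade and Striker monsters for a stage and reports to BP_RealGame when they are all dead.
; MonsterSetting picks a spawn routine by type, passing a fixed 0.1 HP multiplier instead of its Power input.
; Routines randomize spawn points, but RandomInteger bounds leave point D unused and make the random type always Blade.
; Tick prunes dead monsters, then calls ClearStage once the list empties.
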(event EventBeginPlay)

(event EventTick
  (params (DeltaSeconds :type Float%20%28single-precision%29))
  (bind _spawnactors (Variables|Default|GetSpawnActors))
  (if (Variables|Default|GetIsPlaying)
    (Utilities|FlowControl|Sequence
      (:then_0
        (for _array_element _spawnactors
          (if (Variables|/Game/Blueprints/Master/BP_Master.BP_Master_C|GetDeath _array_element)
            (Utilities|Array|RemoveItem _spawnactors _array_element))))
      (:then_1
        (if (<= (Utilities|Array|Length (Variables|Default|GetSpawnActors)) 0)
          (bind _asbp_real_game (Utilities|Casting|CastToBP_RealGame (Game|GetGameMode)))
          (Default|ClearStage _asbp_real_game)
          (Variables|Default|SetIsPlaying false))))))

(fn ConstructionScript)

(fn MonsterSetting
  (params (Type :type E_MonsterType%20Enum :default "NewEnumerator3") (Count :type Integer) (Power :type Float%20%28double-precision%29))
  (bind _returnvalue (Math|Float|MakeLiteralFloat 0.1))
  (switch Utilities|FlowControl|Switch|SwitchonE_MonsterType Type
    (:NewEnumerator3
      (|SpawnRandom Count _returnvalue
        (:Finish
          _)))
    (:NewEnumerator0
      (|SpawnBlade Count _returnvalue
        (:Finish
          _)))
    (:NewEnumerator1
      (|SpawnStriker Count _returnvalue
        (:Finish
          _))))
  (Variables|Default|SetIsPlaying true)
  (return true))
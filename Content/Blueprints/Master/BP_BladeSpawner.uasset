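; BP_BladeSpawner spawns BP_Master actors at randomly chosen spawn points until its tracked list reaches SpawnCount.
; Tick checks the list size and fires a DoOnce, which spawns an actor, adds it to SpawnActors and resets via ResetSpawnerTimer after a short delay.
; Four points are wired, but RandomInteger(3) never selects SpawnPointD.
; Nothing here removes entries from SpawnActors.
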(event Custom|ResetSpawnerTimer
  (Utilities|FlowControl|DoOnce false) ; enters at Reset
)

(event EventBeginPlay)

(event EventTick
  (params (DeltaSeconds :type Float%20%28single-precision%29))
  (if (< (Utilities|Array|Length (Variables|Default|GetSpawnActors)) (Variables|Default|GetSpawnCount))
    (Utilities|FlowControl|DoOnce false
      (:Completed
        (switch int (Math|Random|RandomInteger 3)
          (:0
            (Variables|Default|SetSpawnPoint (Transformation|GetWorldLocation (Variables|Default|GetSpawnPoint_A))))
          (:1
            (Variables|Default|SetSpawnPoint (Transformation|GetWorldLocation (Variables|Default|GetSpawnPoint_B))))
          (:2
            (Variables|Default|SetSpawnPoint (Transformation|GetWorldLocation (Variables|Default|GetSpawnPoint_C))))
          (:3
            (Variables|Default|SetSpawnPoint (Transformation|GetWorldLocation (Variables|Default|GetSpawnPoint_D)))))
        (bind _returnvalue (Game|SpawnActorfromClass "/Game/Blueprints/Master/BP_Master.BP_Master_C" (Math|Transform|MakeTransform (Variables|Default|GetSpawnPoint) "0, 0, 0" "1.000000,1.000000,1.000000") "AdjustIfPossibleButAlwaysSpawn" 0 0))
        (Utilities|Array|AddUnique (Variables|Default|GetSpawnActors) _returnvalue)
        (Utilities|FlowControl|Delay 3.0)
        (CallFunction|ResetSpawnerTimer)))))

(fn ConstructionScript)
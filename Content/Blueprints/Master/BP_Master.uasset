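; BP_Master is an AI-controlled character, apparently a base class, with health, navigation waypoint helpers and combat hit reactions.
; SetFSM mirrors state to the Blackboard and remembers Combat or IDLE to restore after hit timers expire.
; Hit events play montages, some chosen by hit direction, for normal, knockback, launch and air hits.
; Air mode flies briefly; shoot-down forces descent, and landing jumps fall montages to their End section.
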(event EventBeginPlay
  (BlackBoard|SetFSM "NewEnumerator1")
  (bind _asbp_game_instance (Utilities|Casting|CastToBP_GameInstance (Game|GetGameInstance)))
  (Variables|/Script/Engine.CharacterMovementComponent|SetGravityScale (Variables|Character|GetCharacterMovement) (Utilities|Struct|BreakF_GameOption (Variables|/Game/Blueprints/Systems/BP_GameInstance.BP_GameInstance_C|GetGameOption _asbp_game_instance))))

(event EventOnMovementModeChanged
  (params (PrevMovementMode :type EMovementMode%20Enum :default "MOVE_None") (NewMovementMode :type EMovementMode%20Enum :default "MOVE_None") (PrevCustomMode :type Byte :default 0) (NewCustomMode :type Byte :default 0))
  (캐릭터|MovementChanged PrevMovementMode NewMovementMode))

(event EventTick
  (params (DeltaSeconds :type Float%20%28single-precision%29))
  (CallFunction|ShootDownCheck))

(fn ConstructionScript)

(fn GetNextMovePoint
  (bind _waypoints (Variables|Movement|GetWayPoints))
  (if (> (Math|Vector|Distance(Vector) (Transformation|GetActorLocation) (Utilities|Array|Get(acopy) (Variables|Movement|GetWayPoints))) 1e+01) :!label _label
    (return true (Utilities|Array|Get(acopy) (Variables|Movement|GetWayPoints)))
    (else
      (Utilities|Array|RemoveIndex _waypoints)
      (if (<= (Utilities|Array|Length _waypoints) 0)
        (return false "0, 0, 0")
        (else
          (goto _label))))))

(fn GetMovetoLocation
  (return (AI|Components|Blackboard|GetValueasVector (Variables|/Script/AIModule.AIController|GetBlackboard (AI|GetAIController self)) (Utilities|Name|MakeLiteralName "MoveToLocation"))))

(fn FindWayPoint
  (bind _returnvalue (Class|NavigationSystemV1|FindPathtoLocationSynchronously (Class|NavigationSystemV1|GetNavigationSystem) (Transformation|GetActorLocation) (BlackBoard|GetMovetoLocation) 0 0))
  (if (> (Utilities|Array|Length (Variables|/Script/NavigationSystem.NavigationPath|GetPathPoints _returnvalue)) 0)
    (Variables|Movement|SetWayPoints (Variables|/Script/NavigationSystem.NavigationPath|GetPathPoints _returnvalue))
    (return true)
    (else
      (return false))))

(fn SetFSM
  (params (NewFSM :type E_MasterFSM%20Enum :default "NewEnumerator0"))
  (bind _output_get (Variables|Character|SetFSM NewFSM))
  (AI|Components|Blackboard|SetValueasEnum (Variables|/Script/AIModule.AIController|GetBlackboard (AI|GetAIController self)) (Utilities|Name|MakeLiteralName "FSM") _output_get)
  (switch Utilities|FlowControl|Switch|SwitchonE_MasterFSM (Variables|Character|GetFSM)
    (:NewEnumerator4
      _)
    (:NewEnumerator1
      _))
  (Variables|캐릭터|SetPrevFSM (Variables|Character|GetFSM)))

(fn SetHp
  (params (Damage :type Boolean) (Hp :type Float%20%28double-precision%29))
  (if Damage
    (Variables|캐릭터|SetCharacterStatus (Utilities|Struct|MakeF_CharacterState (Math|Float|Clamp(Float) (- (.hp (Variables|캐릭터|GetCharacterStatus)) Hp) 0.0 (.maxhp (Variables|캐릭터|GetCharacterStatus))) (.sp (Variables|캐릭터|GetCharacterStatus)) (.maxhp (Variables|캐릭터|GetCharacterStatus)) (.maxsp (Variables|캐릭터|GetCharacterStatus))))
    (else
      (Variables|캐릭터|SetCharacterStatus (Utilities|Struct|MakeF_CharacterState (Math|Float|Clamp(Float) (+ (.hp (Variables|캐릭터|GetCharacterStatus)) Hp) 0.0 (.maxhp (Variables|캐릭터|GetCharacterStatus))) (.sp (Variables|캐릭터|GetCharacterStatus)) (.maxhp (Variables|캐릭터|GetCharacterStatus)) (.maxsp (Variables|캐릭터|GetCharacterStatus)))))))

(fn FindMovementScale
  (params (TargetLocation :type Vector))
  (bind (_x _y) (Math|Vector|BreakVector TargetLocation))
  (bind _returnvalue (Transformation|GetActorLocation))
  (bind _returnvalue_2 (- (Math|Vector|MakeVector _x _y 0.0) (Math|Vector|MakeVector (.x _returnvalue) (.y _returnvalue) 0.0)))
  (bind _returnvalue_3 (Math|Vector|Normalize _returnvalue_2))
  (return (Math|Float|Lerp 1.0 -1.0 (/ (Math|Trig|RadiansToDegrees (Math|Trig|Acos(Degrees) (Math|Vector|DotProduct _returnvalue_3 (Transformation|GetActorRightVector)))) 1.8e+02)) (Math|Float|Lerp 1.0 -1.0 (/ (Math|Trig|RadiansToDegrees (Math|Trig|Acos(Degrees) (Math|Vector|DotProduct _returnvalue_3 (Transformation|GetActorForwardVector)))) 1.8e+02))))

(fn PlayMontage
  (params (Montage :type Anim%20Montage%20Object%20Reference))
  (bind _returnvalue (Animation|Montage|MontagePlay (Components|SkeletalMesh|GetAnimInstance (Variables|Character|GetMesh)) Montage 1.0 "MontageLength" 0.0 true))
  (return _returnvalue))

(fn JumpMontage
  (params (Section :type Name))
  (bind _returnvalue (Animation|PlayAnimMontage (Animation|GetCurrentMontage :!class /Script/Engine.Character) 1.0 Section))
  (return _returnvalue))

(fn SetHitTime
  (params (time :type Float%20%28double-precision%29))
  (bind _returnvalue (Utilities|Time|SetTimerbyFunctionName 0 (Utilities|String|MakeLiteralString "EndHitTime") time))
  (Variables|Combat|SetHittedTimer _returnvalue))

(fn EndHitTime
  (Utilities|Time|ClearandInvalidateTimerbyHandle (Variables|Combat|GetHittedTimer))
  (BlackBoard|SetFSM (Variables|캐릭터|GetPrevFSM)))

(fn MovementChanged
  (params (Prev :type EMovementMode%20Enum :default "MOVE_None") (New :type EMovementMode%20Enum :default "MOVE_None"))
  (bind _returnvalue (Animation|GetCurrentMontage :!class /Script/Engine.Character))
  (Utilities|FlowControl|Sequence
    (:then_0
      (if (Utilities|Enum|Equal(Enum) New "MOVE_Walking")
        (if (or (Utilities|Enum|Equal(Enum) Prev "MOVE_Falling") (Utilities|Enum|Equal(Enum) Prev "MOVE_Flying"))
          (Variables|Combat|SetIsShootDown false)
          (if (or (== _returnvalue "/Game/Animations/Montage/Blade/Hit/AM_FallDown_F.AM_FallDown_F") (== _returnvalue "/Game/Animations/Montage/Blade/Hit/AM_FallDown_B.AM_FallDown_B"))
            (bind _montagetime (Animation|JumpMontage "End"))
            (Combat|SetHitTime _montagetime)))))))

(fn ShootDownCheck
  (if (Variables|Combat|GetIsShootDown)
    (Character|LaunchCharacter "0.000000,0.000000,-500.000000" false false)))

(event EventPlayAirMode
  (Pawn|Components|CharacterMovement|SetMovementMode (Variables|Character|GetCharacterMovement) "MOVE_Flying" 0)
  (bind _returnvalue (Utilities|Time|SetTimerbyEvent (delegate EventEndAirMode) 3.0))
  (Variables|Combat|SetAirModeTimer _returnvalue))

(event EventEndAirMode
  (Pawn|Components|CharacterMovement|SetMovementMode (Variables|Character|GetCharacterMovement) "MOVE_Falling" 0))

(event EventHitReactionFallDownEnd
  (bind _montagetime (Animation|PlayMontage "/Game/Animations/Montage/Blade/Hit/AM_FallDownHit.AM_FallDownHit"))
  (Combat|SetHitTime _montagetime))

(event EventHitReactionKnockBack
  (params (HitPoint :type Vector :default "0, 0, 0"))
  (Transformation|SetActorRotation (Math|Rotator|FindLookatRotation (Transformation|GetActorLocation) HitPoint))
  (bind _montagetime (Animation|PlayMontage "/Game/Animations/Montage/Blade/Hit/AM_KnockBack.AM_KnockBack"))
  (Combat|SetHitTime _montagetime))

(event EventHitReactionShootDown
  (params (HitPoint :type Vector :default "0, 0, 0"))
  (Variables|Combat|SetIsShootDown true)
  (CallFunction|EndAirMode)
  (bind _montagetime (Animation|PlayMontage "/Game/Animations/Montage/Blade/Hit/AM_FallDown_B.AM_FallDown_B"))
  (Combat|SetHitTime _montagetime)
  (Utilities|Time|PauseTimerbyHandle (Variables|Combat|GetHittedTimer)))

(event EventHitReactionAir
  (params (HitPoint :type Vector :default "0, 0, 0"))
  (BlackBoard|SetFSM "NewEnumerator0")
  (bind _montagetime (Animation|JumpMontage "Hitting"))
  (Combat|SetHitTime _montagetime))

(event EventHitReactionNormal
  (params (HitPoint :type Vector :default "0, 0, 0"))
  (bind _rightsacle (이동|FindMovementScale HitPoint))
  (bind _forwardscale (이동|FindMovementScale HitPoint))
  (BlackBoard|SetFSM "NewEnumerator0")
  (if (> _forwardscale 0.5)
    (bind _montagetime (Animation|PlayMontage "/Game/Animations/Montage/Blade/Hit/AM_DefaultHit_F.AM_DefaultHit_F"))
    (Combat|SetHitTime _montagetime)
    (elif (< _forwardscale -0.5)
      (bind _montagetime_2 (Animation|PlayMontage "/Game/Animations/Montage/Blade/Hit/AM_DefaultHit_B.AM_DefaultHit_B"))
      (Combat|SetHitTime _montagetime_2)
      (elif (> _rightsacle 0.5)
        (bind _montagetime_3 (Animation|PlayMontage "/Game/Animations/Montage/Blade/Hit/AM_DefaultHit_R.AM_DefaultHit_R"))
        (Combat|SetHitTime _montagetime_3)
        (elif (< _rightsacle -0.5)
          (bind _montagetime_4 (Animation|PlayMontage "/Game/Animations/Montage/Blade/Hit/AM_DefaultHit_L.AM_DefaultHit_L"))
          (Combat|SetHitTime _montagetime_4))))))

(event Game|Damage|EventAnyDamage
  (params (Damage :type Float%20%28single-precision%29) (DamageType :type Damage%20Type%20Object%20Reference) (InstigatedBy :type Controller%20Object%20Reference) (DamageCauser :type Actor%20Object%20Reference))
  (캐릭터|SetHp true Damage))

(event EventHitReactionUpper
  (params (HitPoint :type Vector :default "0, 0, 0"))
  (Utilities|FlowControl|Sequence
    (:then_0
      (BlackBoard|SetFSM "NewEnumerator0"))
    (:then_1
      (if (> (.ForwardScale (이동|FindMovementScale HitPoint)) 0.0)
        (bind _montagetime (Animation|PlayMontage "/Game/Animations/Montage/Blade/Hit/AM_FallDown_F.AM_FallDown_F"))
        (Combat|SetHitTime _montagetime)
        (Utilities|Time|PauseTimerbyHandle (Variables|Combat|GetHittedTimer))
        (else
          (bind _montagetime_2 (Animation|PlayMontage "/Game/Animations/Montage/Blade/Hit/AM_FallDown_B.AM_FallDown_B"))
          (Combat|SetHitTime _montagetime_2)
          (Utilities|Time|PauseTimerbyHandle (Variables|Combat|GetHittedTimer)))))))

(fn Moveto
  (params (MoveToLocation :type Vector :default "0, 0, 0"))
  (if (Utilities|Array|IsEmpty (Variables|Movement|GetWayPoints))
    (bind _complete (Movement|FindWayPoint))
    (if (not _complete)
      (return true))))
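; BP_Knight is a Knight character Blueprint that handles player-driven movement and look through Enhanced Input actions.
; Forward and right actions scale the actor's own direction vectors and feed them into CharacterMovement as input vectors.
; Look actions drive controller yaw and pitch, with pitch inverted.
; BeginPlay, Tick, overlap and construction script hold no logic.
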(event EventBeginPlay)

(event Collision|EventActorBeginOverlap
  (params (OtherActor :type Actor%20Object%20Reference)))

(event EventTick
  (params (DeltaSeconds :type Float%20%28single-precision%29)))

(fn ConstructionScript)

(event Input|EnhancedActionEvents|EnhancedInputActionIA_MoveForward
  (params (ActionValue :type Float%20%28double-precision%29) (ElapsedSeconds :type Float%20%28double-precision%29) (TriggeredSeconds :type Float%20%28double-precision%29) (InputAction :type Input%20Action%20Object%20Reference :default "/Game/InputSystem/IA_MoveForward.IA_MoveForward"))
  ;[1 1 1] MovementInput
  (:Triggered
    (Class|PawnMovementComponent|AddInputVector (Variables|Character|GetCharacterMovement) (* (Transformation|GetActorForwardVector) ActionValue) false)))

(event Input|EnhancedActionEvents|EnhancedInputActionIA_MoveRight
  (params (ActionValue :type Float%20%28double-precision%29) (ElapsedSeconds :type Float%20%28double-precision%29) (TriggeredSeconds :type Float%20%28double-precision%29) (InputAction :type Input%20Action%20Object%20Reference :default "/Game/InputSystem/IA_MoveRight.IA_MoveRight"))
  ;[1 1 1] MovementInput
  (:Triggered
    (Class|PawnMovementComponent|AddInputVector (Variables|Character|GetCharacterMovement) (* (Transformation|GetActorRightVector) ActionValue) false)))

(event Input|EnhancedActionEvents|EnhancedInputActionIA_LookUp
  (params (ActionValue :type Float%20%28double-precision%29) (ElapsedSeconds :type Float%20%28double-precision%29) (TriggeredSeconds :type Float%20%28double-precision%29) (InputAction :type Input%20Action%20Object%20Reference :default "/Game/InputSystem/IA_LookUp.IA_LookUp"))
  ;[1 1 1] MovementInput
  (:Triggered
    (Pawn|Input|AddControllerPitchInput (* ActionValue -1.0))))

(event Input|EnhancedActionEvents|EnhancedInputActionIA_LookRight
  (params (ActionValue :type Float%20%28double-precision%29) (ElapsedSeconds :type Float%20%28double-precision%29) (TriggeredSeconds :type Float%20%28double-precision%29) (InputAction :type Input%20Action%20Object%20Reference :default "/Game/InputSystem/IA_LookRight.IA_LookRight"))
  ;[1 1 1] MovementInput
  (:Triggered
    (Pawn|Input|AddControllerYawInput ActionValue)))
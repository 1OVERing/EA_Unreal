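; BP_BladeSpawner spawns BP_Blade actors and tracks them in SpawnActors, up to SpawnCount.
; Tick feeds a DoOnce while below the count, so each spawn waits for ResetSpawnerTimer to re-arm it.
; Blades appear above a random navigable point within the Box's X extent of the spawner, or at a fixed world position if none is found.
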(event Custom|ResetSpawnerTimer
  (Utilities|FlowControl|DoOnce false) ; enters at Reset
)

(event EventBeginPlay)

(event EventTick
  (params (DeltaSeconds :type Float%20%28single-precision%29))
  (if (< (Utilities|Array|Length (Variables|Default|GetSpawnActors)) (Variables|Default|GetSpawnCount))
    (Utilities|FlowControl|DoOnce false
      (:Completed
        (bind (_randomlocation _returnvalue) (Class|NavigationSystemV1|GetRandomLocationinNavigableRadius (Transformation|GetActorLocation) (.x (Variables|/Script/Engine.BoxComponent|GetBoxExtent (Variables|Default|GetBox))) 0 0))
        (if _returnvalue
          (bind _returnvalue_2 (Game|SpawnActorfromClass "/Game/Blueprints/Blade/BP_Blade.BP_Blade_C" (Math|Transform|MakeTransform (+ _randomlocation "0.000000,0.000000,200.000000") "0, 0, 0" "1.000000,1.000000,1.000000") "AlwaysSpawn" 0 0))
          (Utilities|Array|AddUnique (Variables|Default|GetSpawnActors) _returnvalue_2)
          (else
            (bind _returnvalue_3 (Game|SpawnActorfromClass "/Game/Blueprints/Blade/BP_Blade.BP_Blade_C" (Math|Transform|MakeTransform "300.000000,300.000000,300.000000" "0, 0, 0" "1.000000,1.000000,1.000000") "AlwaysSpawn" 0 0))
            (Utilities|Array|AddUnique (Variables|Default|GetSpawnActors) _returnvalue_3)))))))

(fn ConstructionScript)
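; BP_BladeAtack6 is a blade attack actor that deals an area hit around its own location one second after BeginPlay.
; A multi-sphere trace applies normal-type damage to each hit and sends actors implementing BPI_ActionInteraction a knockback montage message.
; The GameInstance check that sets the trace's debug draw type from the attack debug option is disconnected, so it never runs.
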(event EventBeginPlay
  (bind _returnvalue (Transformation|GetActorLocation))
  (Utilities|FlowControl|Delay 1.0)
  (Utilities|FlowControl|Sequence
    (:then_1
      (bind (_outhits _returnvalue_2) (Collision|MultiSphereTraceByChannel _returnvalue _returnvalue 4e+02 "TraceTypeQuery4" false 0 (Variables|Default|GetDrawType) true "(R=1.000000,G=0.000000,B=0.000000,A=1.000000)" "(R=0.000000,G=1.000000,B=0.000000,A=1.000000)" 1.0))
      (if _returnvalue_2
        (for _array_element _outhits
          (Game|Damage|ApplyDamage (.HitActor (Collision|BreakHitResult _array_element)) 25.0 0 self "/Game/Blueprints/DTBP/DTBP_Normal.DTBP_Normal_C")
          (if (Utilities|DoesObjectImplementInterface (.HitActor (Collision|BreakHitResult _array_element)) "/Game/Blueprints/Interface/BPI_ActionInteraction.BPI_ActionInteraction_C")
            (Class|BPIActionInteraction|PlayActionMontage(Message) (.HitActor (Collision|BreakHitResult _array_element)) false "/Game/Animations/Montage/Assassin/Hit/AM_Hit_KnockBack.AM_Hit_KnockBack")))))))

(event Collision|EventActorBeginOverlap
  (params (OtherActor :type Actor%20Object%20Reference)))

(event EventTick
  (params (DeltaSeconds :type Float%20%28single-precision%29)))

(fn ConstructionScript)
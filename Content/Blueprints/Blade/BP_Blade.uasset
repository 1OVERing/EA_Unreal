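; BP_Blade is an AI-controlled character (AIC_Blade) with modular meshes following the main mesh's pose and hit-driven aerial reactions.
; Damage types trigger either a timed flying air mode or a shoot-down that launches it downward until a ground trace reads close.
; Tick reads blackboard move targets, builds a navmesh path and turns toward waypoints while idle.
; Timelines ease MovementScale in and out; translation is not applied here.
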(event Custom|ShootDown
  (Variables|이동|SetIsShootDown true)
  (CallFunction|AirModeEnd))

(event Custom|StartMovementScale
  (switch Utilities|FlowControl|Switch|SwitchonE_BladeFSM (Variables|FSM|GetFSM)
    (:NewEnumerator0
      (bind _alpha (Timeline|타임라인 PlayFromStart)
        (:Update
          (Variables|Movement|SetMovementScale (Math|Vector2D|MakeVector2D 0.0 (Math|Float|Lerp 0.0 1.0 _alpha))))))))

(event Custom|EndedMovementScale
  (Utilities|FlowControl|Sequence
    (:then_0
      (Variables|이동|SetPrevMovementScale (Variables|Movement|GetMovementScale)))
    (:then_1
      (bind _alpha (Timeline|TL_EndedMove PlayFromStart)
        (:Update
          (Variables|Movement|SetMovementScale (Math|Vector2D|MakeVector2D (Math|Float|Lerp (.x (Variables|이동|GetPrevMovementScale)) 0.0 _alpha) (Math|Float|Lerp (.y (Variables|이동|GetPrevMovementScale)) 0.0 _alpha))))))))

(event EventBeginPlay
  (Utilities|FlowControl|Sequence
    (:then_0
      (|Node_DefaultSetting))))

(event Collision|EventActorBeginOverlap
  (params (OtherActor :type Actor%20Object%20Reference)))

(event EventTick
  (params (DeltaSeconds :type Float%20%28single-precision%29))
  (Movement|UpdateShootDown)
  (이동|UpdateMoveto))

(event Game|Damage|EventAnyDamage
  (params (Damage :type Float%20%28single-precision%29) (DamageType :type Damage%20Type%20Object%20Reference) (InstigatedBy :type Controller%20Object%20Reference) (DamageCauser :type Actor%20Object%20Reference))
  (Utilities|FlowControl|Sequence
    (:then_0
      (Utilities|Casting|CastToDTBP_AirAttack DamageType)
      (CallFunction|PlayAirMode))
    (:then_1
      (Utilities|Casting|CastToDTBP_ShootDown DamageType)
      (CallFunction|ShootDown))))

(event EventAirModeEnd
  (if (> (Movement|LandingCheck) 5e+01)
    (Pawn|Components|CharacterMovement|SetMovementMode (Variables|Character|GetCharacterMovement) "MOVE_Falling" 0)
    (else
      (Pawn|Components|CharacterMovement|SetMovementMode (Variables|Character|GetCharacterMovement) "MOVE_Walking" 0)))
  (Variables|Movement|SetAirMode false))

(event EventPlayAirMode
  (Pawn|Components|CharacterMovement|SetMovementMode (Variables|Character|GetCharacterMovement) "MOVE_Flying" 0)
  (Variables|Movement|SetAirMode true)
  (Timeline|EndAirModeTimer PlayFromStart
    (:Finished
      (CallFunction|AirModeEnd))))

(fn ConstructionScript
  (Components|SkinnedMesh|SetLeaderPoseComponent (Variables|Default|GetSK_BotBody) (Variables|Character|GetMesh) true false)
  (Variables|Default|SetAIControllerClass "/Game/Blueprints/Blade/AI/AIC_Blade.AIC_Blade_C"))

(fn LandingCheck
  (bind _returnvalue (Transformation|GetActorLocation))
  (bind _capsulecomponent (Variables|Collision|GetCapsuleComponent))
  (bind _returnvalue_2 (Components|Capsule|GetScaledCapsuleHalfHeight _capsulecomponent))
  (bind _returnvalue_3 (- (.z _returnvalue) _returnvalue_2))
  (Utilities|FlowControl|Sequence
    (:then_0
      (bind _asbp_game_instance (Utilities|Casting|CastToBP_GameInstance (Game|GetGameInstance)))
      (if (.OnAttackDebugTrace (Utilities|Struct|BreakF_GameOption (Variables|/Game/Blueprints/Systems/BP_GameInstance.BP_GameInstance_C|GetGameOption _asbp_game_instance)))
        (LocalVariables|SetDrawType "ForDuration")
        (else
          (LocalVariables|SetDrawType "None"))))
    (:then_1
      (bind (_outhit _returnvalue_4) (Collision|LineTraceByChannel (Math|Vector|MakeVector (.x _returnvalue) (.y _returnvalue) _returnvalue_3) (Math|Vector|MakeVector (.x _returnvalue) (.y _returnvalue) (- _returnvalue_3 2e+03)) "TraceTypeQuery1" false 0 (LocalVariables|GetDrawType)))
      (if _returnvalue_4
        (return (.Distance (Collision|BreakHitResult _outhit)))
        (else
          (return 1e+04))))))

(fn UpdateShootDown
  (if (Variables|이동|GetIsShootDown)
    (if (> (Movement|LandingCheck) 1e+02)
      (Character|LaunchCharacter "0.000000,0.000000,-1000.000000" false false)
      (else
        (Variables|이동|SetIsShootDown false)))))

(fn ChangedFSM
  (params (NewFSM :type E_BladeFSM%20Enum :default "NewEnumerator0")))

(fn GetMoveto
  (return (ScalableFloat|GetValueasBool (Variables|/Script/AIModule.AIController|GetBlackboard (AI|GetAIController self)) (Utilities|Name|MakeLiteralName "MoveTo"))))

(fn GetMovetoLocation
  (return (AI|Components|Blackboard|GetValueasVector (Variables|/Script/AIModule.AIController|GetBlackboard (AI|GetAIController self)) (Utilities|Name|MakeLiteralName "MoveToLocation"))))

(fn UpdateMoveto
  (if (BlackBoard|GetMoveto)
    (if (> (Math|Vector|Distance(Vector) (BlackBoard|GetMovetoLocation) (Transformation|GetActorLocation)) 1e+02)
      (if (이동|HavetoMove)
        (switch Utilities|FlowControl|Switch|SwitchonE_BladeFSM (Variables|FSM|GetFSM)
          (:NewEnumerator0
            (이동|IdleMove 0.0 1e+02)))
        (else
          (bind _returnvalue (Class|NavigationSystemV1|FindPathtoLocationSynchronously (Class|NavigationSystemV1|GetNavigationSystem) (Transformation|GetActorLocation) (BlackBoard|GetMovetoLocation) 0 0))
          (if (> (Utilities|Array|Length (Variables|/Script/NavigationSystem.NavigationPath|GetPathPoints _returnvalue)) 0)
            (Variables|이동|SetWayPoints (Variables|/Script/NavigationSystem.NavigationPath|GetPathPoints _returnvalue))
            (CallFunction|StartMovementScale)
            (else
              (이동|ClearMoveParams)))))
      (else
        (이동|ClearMoveParams)))))

(fn SetMoveto
  (params (New%20Value :type Boolean))
  (AI|Components|Blackboard|SetValueasBool (Variables|/Script/AIModule.AIController|GetBlackboard (AI|GetAIController self)) (Utilities|Name|MakeLiteralName "MoveTo") New%20Value))

(fn SetMovetoLocation
  (params (NewLocation :type Vector))
  (AI|Components|Blackboard|SetValueasVector (Variables|/Script/AIModule.AIController|GetBlackboard (AI|GetAIController self)) (Utilities|Name|MakeLiteralName "MoveToLocation") NewLocation))

(fn ClearMoveParams
  (BlackBoard|SetMoveto false)
  (BlackBoard|SetMovetoLocation "0, 0, 0")
  (Utilities|Array|Clear (Variables|이동|GetWayPoints))
  (CallFunction|EndedMovementScale))

(fn HavetoMove
  (return (> (Utilities|Array|Length (Variables|이동|GetWayPoints)) 0)))

(fn GetNextMovePoint
  (bind _waypoints (Variables|이동|GetWayPoints))
  (if (> (Math|Vector|Distance(Vector) (Transformation|GetActorLocation) (Utilities|Array|Get(acopy) (Variables|이동|GetWayPoints))) 1e+02) :!label _label
    (return true (Utilities|Array|Get(acopy) (Variables|이동|GetWayPoints)))
    (else
      (Utilities|Array|RemoveIndex _waypoints)
      (if (<= (Utilities|Array|Length _waypoints) 0)
        (return false "0, 0, 0")
        (else
          (goto _label))))))

(fn IdleMove
  (params (MaginAngle :type Float%20%28double-precision%29) (RotationSpeed :type Float%20%28double-precision%29))
  (bind _returnvalue (Utilities|Time|GetWorldDeltaSeconds))
  (bind _returnvalue_2 (Transformation|GetActorLocation))
  (bind _returnvalue_3 (Transformation|GetActorForwardVector))
  (bind _returnvalue_4 (* RotationSpeed _returnvalue))
  (bind (_validwaypoint _nextmovepoint) (이동|GetNextMovePoint))
  (if _validwaypoint
    (if (> (Math|Trig|RadiansToDegrees (Math|Trig|Acos(Degrees) (Math|Vector|DotProduct (Math|Vector|Normalize (- (Math|Vector|MakeVector (.X (Math|Vector|BreakVector _nextmovepoint)) (.Y (Math|Vector|BreakVector _nextmovepoint)) 0.0) (Math|Vector|MakeVector (.x _returnvalue_2) (.y _returnvalue_2) 0.0))) _returnvalue_3))) MaginAngle)
      (if (< (.z (Math|Vector|CrossProduct _returnvalue_3 (Math|Vector|Normalize (- (Math|Vector|MakeVector (.X (Math|Vector|BreakVector _nextmovepoint)) (.Y (Math|Vector|BreakVector _nextmovepoint)) 0.0) (Math|Vector|MakeVector (.x _returnvalue_2) (.y _returnvalue_2) 0.0))))) 0.0)
        (Class|Actor|AddActorWorldRotation (Math|Rotator|MakeRotator 0.0 0.0 (* _returnvalue_4 -1.0)))
        (else
          (Class|Actor|AddActorWorldRotation (Math|Rotator|MakeRotator 0.0 0.0 _returnvalue_4)))))
    (else
      (이동|ClearMoveParams))))
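; Player character with switchable dagger and katana, built from modular meshes following the main mesh via leader pose.
; Enhanced Input drives movement, equip and weapon-change states, with montages for equipping, jumping, dagger combos and directional slides or rolls.
; Weapon events reattach meshes between sockets.
; Falling adds manual air steering and trace-gated jump loops; a test key halts falls, restoring gravity by timeline, while damage handling is only a stub.
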(event Game|Damage|EventAnyDamage
  (params (Damage :type Float%20%28single-precision%29) (DamageType :type Damage%20Type%20Object%20Reference) (InstigatedBy :type Controller%20Object%20Reference) (DamageCauser :type Actor%20Object%20Reference))
  (Utilities|Casting|CastToDTBP_Damage DamageType))

(event EventTick
  (params (DeltaSeconds :type Float%20%28single-precision%29))
  (if (AI|Components|NavMovement|IsFalling (Variables|Character|GetCharacterMovement))
    (Movement|UpdateJumpingMove)))

(fn ConstructionScript
  (Components|SkinnedMesh|SetLeaderPoseComponent (Variables|Default|GetSK_Shoes) (Variables|Character|GetMesh) true false)
  (FSM|SetMovement "NewEnumerator0" true)
  (FSM|SetWeaponType "NewEnumerator0" true)
  (FSM|SetWeaponEquip "NewEnumerator1" true))

(fn UpdateJumpingMove
  (if (not (Variables|Movement|GetDontMove))
    (Transformation|SetActorLocation (+ (Transformation|GetActorLocation) (* (* (* (Math|Vector|GetForwardVector (Math|Rotator|MakeRotator 0.0 0.0 (.yaw (Pawn|GetControlRotation :!class /Script/Engine.Pawn)))) (.y (Variables|Movement|GetInputScale))) (Utilities|Time|GetWorldDeltaSeconds)) (Variables|Movement|GetCharacterJumpMoveSpeed))) true false)
    (Transformation|SetActorLocation (+ (Transformation|GetActorLocation) (* (* (* (Math|Vector|GetRightVector (Pawn|GetControlRotation :!class /Script/Engine.Pawn)) (.x (Variables|Movement|GetInputScale))) (Utilities|Time|GetWorldDeltaSeconds)) (Variables|Movement|GetCharacterJumpMoveSpeed))) true false)))

(fn CharacterLanding
  (bind _returnvalue (Transformation|GetActorLocation))
  (bind _capsulecomponent (Variables|Collision|GetCapsuleComponent))
  (bind _returnvalue_2 (Components|Capsule|GetScaledCapsuleHalfHeight _capsulecomponent))
  (bind _returnvalue_3 (- (.z _returnvalue) _returnvalue_2))
  (bind (_outhit _returnvalue_4) (Collision|LineTraceByChannel (Math|Vector|MakeVector (.x _returnvalue) (.y _returnvalue) _returnvalue_3) (Math|Vector|MakeVector (.x _returnvalue) (.y _returnvalue) (- _returnvalue_3 2e+03)) "TraceTypeQuery1" false 0 "ForDuration"))
  (if _returnvalue_4
    (return (.Distance (Collision|BreakHitResult _outhit)))
    (else
      (return 1e+04))))

(fn GetCurrentAnimMontage
  (bind _mesh (Variables|Character|GetMesh))
  (bind _returnvalue (Components|SkeletalMesh|GetAnimInstance _mesh))
  (bind _returnvalue_2 (Animation|Montage|GetCurrentActiveMontage _returnvalue))
  (return _returnvalue_2 (Utilities|GetObjectName _returnvalue_2) (Utilities|String|ToString(Name) (Animation|Montage|MontageGetCurrentSection _returnvalue _returnvalue_2))))

(fn CurrentMontageCheck
  (params (CheckMontage :type Anim%20Montage%20Object%20Reference))
  (return (== CheckMontage (Animation|GetCurrentMontage :!class /Script/Engine.Character))))

(fn SetMovement
  (params (NewMovement :type E_Movement%20Enum :default "NewEnumerator0") (Enforce :type Boolean))
  (if Enforce
    (switch Utilities|FlowControl|Switch|SwitchonE_Movement (Variables|FSM|GetCurrentMovement) :!label _label
      (:NewEnumerator0
        (switch Utilities|FlowControl|Switch|SwitchonE_Movement NewMovement))
      (:NewEnumerator1
        (switch Utilities|FlowControl|Switch|SwitchonE_Movement NewMovement))
      (:NewEnumerator2
        (switch Utilities|FlowControl|Switch|SwitchonE_Movement NewMovement)))
    (elif (Utilities|Enum|NotEqual(Enum) NewMovement (Variables|FSM|GetCurrentMovement))
      (goto _label))))

(fn SetWeaponType
  (params (NewType :type E_WeaponType%20Enum :default "NewEnumerator0") (Enforce :type Boolean))
  (if Enforce
    (Variables|FSM|SetCurrent_WeaponType NewType :!label _label)
    (elif (Utilities|Enum|NotEqual(Enum) NewType (Variables|FSM|GetCurrent_WeaponType))
      (goto _label))))

(fn SetWeaponEquip
  (params (NewEquip :type E_WeaponEquip%20Enum :default "NewEnumerator1") (Enforce :type Boolean))
  (if Enforce
    (Variables|FSM|SetCurrent_WeaponEquip NewEquip :!label _label)
    (switch Utilities|FlowControl|Switch|SwitchonE_WeaponType (Variables|FSM|GetCurrent_WeaponType)
      (:NewEnumerator0
        (switch Utilities|FlowControl|Switch|SwitchonE_WeaponEquip (Variables|FSM|GetCurrent_WeaponEquip)
          (:NewEnumerator1
            (Animation|PlayAnimMontage "/Game/Animations/Montage/DAGGER/Movement/AM_DaggerEquip.AM_DaggerEquip" 1.0 "UnEquip")
            (Variables|Default|SetbUseControllerRotationYaw false))
          (:NewEnumerator0
            (Animation|PlayAnimMontage "/Game/Animations/Montage/DAGGER/Movement/AM_DaggerEquip.AM_DaggerEquip" 1.0 "Equip")
            (Variables|Default|SetbUseControllerRotationYaw true))))
      (:NewEnumerator1
        (switch Utilities|FlowControl|Switch|SwitchonE_WeaponEquip (Variables|FSM|GetCurrent_WeaponEquip)
          (:NewEnumerator1
            (Animation|PlayAnimMontage "/Game/Animations/Montage/KATANA/AM_KatanaEquip.AM_KatanaEquip" 1.0 "UnEquip")
            (Variables|Default|SetbUseControllerRotationYaw false))
          (:NewEnumerator0
            (Animation|PlayAnimMontage "/Game/Animations/Montage/KATANA/AM_KatanaEquip.AM_KatanaEquip" 1.0 "Equip")
            (Variables|Default|SetbUseControllerRotationYaw true)))))
    (elif (Utilities|Enum|NotEqual(Enum) NewEquip (Variables|FSM|GetCurrent_WeaponEquip))
      (goto _label))))

(fn Jumping
  (params (Loop :type Boolean))
  (if Loop
    (Animation|PlayAnimMontage "/Game/Animations/Montage/DAGGER/Movement/AM_DaggerJump.AM_DaggerJump" 1.0 "Loop")
    (Variables|Movement|SetJumpStartPositionZ (.z (Transformation|GetActorLocation)))
    (else
      (Animation|PlayAnimMontage "/Game/Animations/Montage/DAGGER/Movement/AM_DaggerJump.AM_DaggerJump" 1.0 "")
      (Variables|Movement|SetJumpStartPositionZ (.z (Transformation|GetActorLocation))))))

(fn MovementUpdateTriggered
  (params (InputPin :type Vector%202D%20Structure))
  (bind (_x _y) (Math|Vector2D|BreakVector2D InputPin))
  (Utilities|FlowControl|Sequence
    (:then_0
      (Variables|Movement|SetInputScale InputPin)
      (if (Variables|Movement|GetSprint)
        (Variables|Movement|SetInputScale (* (Variables|Movement|GetInputScale) "(X=2.000000,Y=2.000000)"))
        (FSM|SetMovement "NewEnumerator2" false)
        (else
          (FSM|SetMovement "NewEnumerator1" false))))
    (:then_1
      (Transformation|SetActorRotation (Math|Conversions|RotationFromXVector (+ (* (Math|Vector|GetForwardVector (Pawn|GetControlRotation :!class /Script/Engine.Pawn)) _y) (* _x (Math|Vector|GetRightVector (Pawn|GetControlRotation :!class /Script/Engine.Pawn)))))))))

(fn MovementUpdateCompleted
  (Variables|Movement|SetSprint false)
  (FSM|SetMovement "NewEnumerator0" false)
  (CallFunction|ResetInputSacle))

(fn NextAttackPlay
  (if (Variables|Default|GetNextAttackCheck)
    (switch Utilities|FlowControl|Switch|SwitchonE_WeaponType (Variables|FSM|GetCurrent_WeaponType)
      (:NewEnumerator0
        (Math|Integer|IncrementInt (Variables|Default|GetCurrentCombo)
          (:%20%20
            (Ability|Animation|MontageJumptoSection (Components|SkeletalMesh|GetAnimInstance (Variables|Character|GetMesh)) (Utilities|String|StringToName (Utilities|String|ToString(Integer) (Variables|Default|GetCurrentCombo))) 0)
            (Variables|Default|SetNextAttackCheck false)))))))

(event Input|EnhancedActionEvents|EnhancedInputActionIA_Movement
  (params (ActionValue :type Vector%202D%20Structure) (ElapsedSeconds :type Float%20%28double-precision%29) (TriggeredSeconds :type Float%20%28double-precision%29) (InputAction :type Input%20Action%20Object%20Reference :default "/Game/InputSystem/IA_Movement.IA_Movement"))
  ;[1 1 1] Movement
  (:Triggered
    (이동|MovementUpdateTriggered ActionValue))
  (:Completed
    (이동|MovementUpdateCompleted)))

(event Input|EnhancedActionEvents|EnhancedInputActionIA_Look
  (params (ActionValue :type Vector%202D%20Structure) (ElapsedSeconds :type Float%20%28double-precision%29) (TriggeredSeconds :type Float%20%28double-precision%29) (InputAction :type Input%20Action%20Object%20Reference :default "/Game/InputSystem/IA_Look.IA_Look"))
  ;[1 1 1] Movement
)

(event Input|EnhancedActionEvents|EnhancedInputActionIA_LMouse
  (params (ActionValue :type Boolean) (ElapsedSeconds :type Float%20%28double-precision%29) (TriggeredSeconds :type Float%20%28double-precision%29) (InputAction :type Input%20Action%20Object%20Reference :default "/Game/InputSystem/IA_LMouse.IA_LMouse"))
  (bind _inputscale (Variables|Movement|GetInputScale))
  (:Started
    (switch Utilities|FlowControl|Switch|SwitchonE_WeaponEquip (Variables|FSM|GetCurrent_WeaponEquip)
      (:NewEnumerator0
        (if (Variables|Default|GetAttacking)
          (Variables|Default|SetNextAttackCheck true)
          (elif (not (> (.x _inputscale) 0.0)) ; Right
            (if (not (< (.x _inputscale) 0.0)) ; Left
              (if (not (< (.y _inputscale) 0.0)) ; Back
                (Animation|PlayAnimMontage "/Game/Animations/Montage/DAGGER/Attack/AM_DaggerAttackCombo_F.AM_DaggerAttackCombo_F" 1.0 "None")
                (Variables|Default|SetCurrentCombo 0)
                (Variables|Default|SetAttacking true)))))))))

(event Input|MouseEvents|RightMouseButton
  (params (Key :type Key%20Structure :default "None"))
  (bind _charactermovement (Variables|Character|GetCharacterMovement))
  ;[1 1 1] 테스트 키
  (:Pressed
    (if (AI|Components|NavMovement|IsFalling (Variables|Character|GetCharacterMovement))
      (Animation|Montage|PlayMontage (Variables|Character|GetMesh) "/Game/Animations/Montage/DAGGER/Movement/AM_DaggerJump.AM_DaggerJump" 1.0 0.0 "Loop"
        (:then
          (Variables|Movement|SetIsAirMode true)
          (Variables|/Script/Engine.CharacterMovementComponent|SetGravityScale _charactermovement 0.0)
          (Variables|/Script/Engine.MovementComponent|SetVelocity _charactermovement "0, 0, 0")
          (CallFunction|ResetGravity)
          (Variables|Movement|SetDontMove true))))))

(event Input|EnhancedActionEvents|EnhancedInputActionIA_Equip
  (params (ActionValue :type Boolean) (ElapsedSeconds :type Float%20%28double-precision%29) (TriggeredSeconds :type Float%20%28double-precision%29) (InputAction :type Input%20Action%20Object%20Reference :default "/Game/InputSystem/IA_Equip.IA_Equip"))
  (:Started
    (if (Math|Boolean|NANDBoolean (Animation|CurrentMontageCheck "/Game/Animations/Montage/DAGGER/Movement/AM_DaggerEquip.AM_DaggerEquip") (Animation|CurrentMontageCheck "/Game/Animations/Montage/KATANA/AM_KatanaEquip.AM_KatanaEquip"))
      (switch Utilities|FlowControl|Switch|SwitchonE_WeaponEquip (Variables|FSM|GetCurrent_WeaponEquip)
        (:NewEnumerator1
          (FSM|SetWeaponEquip "NewEnumerator0" false))
        (:NewEnumerator0
          (FSM|SetWeaponEquip "NewEnumerator1" false))))))

(event Input|EnhancedActionEvents|EnhancedInputActionIA_Jump
  (params (ActionValue :type Boolean) (ElapsedSeconds :type Float%20%28double-precision%29) (TriggeredSeconds :type Float%20%28double-precision%29) (InputAction :type Input%20Action%20Object%20Reference :default "/Game/InputSystem/IA_Jump.IA_Jump"))
  (:Started
    (Movement|Jumping false)))

(event Input|EnhancedActionEvents|EnhancedInputActionIA_Sprint
  (params (ActionValue :type Boolean) (ElapsedSeconds :type Float%20%28double-precision%29) (TriggeredSeconds :type Float%20%28double-precision%29) (InputAction :type Input%20Action%20Object%20Reference :default "/Game/InputSystem/IA_Sprint.IA_Sprint"))
  (:Started
    (Variables|Movement|SetSprint true)
    (switch Utilities|FlowControl|Switch|SwitchonE_WeaponType (Variables|FSM|GetCurrent_WeaponType)
      (:NewEnumerator0
        (switch Utilities|FlowControl|Switch|SwitchonE_WeaponEquip (Variables|FSM|GetCurrent_WeaponEquip)
          (:NewEnumerator0
            (if (not (Animation|CurrentMontageCheck "/Game/Animations/Montage/DAGGER/Movement/AM_DaggerRolling.AM_DaggerRolling"))
              (if (Animation|CurrentMontageCheck "/Game/Animations/Montage/DAGGER/Movement/AM_DaggerSlide.AM_DaggerSlide")
                (Variables|Movement|SetCanRolling true)
                (else
                  (CallFunction|PlaySliding)))))))
      (:NewEnumerator1
        (switch Utilities|FlowControl|Switch|SwitchonE_WeaponEquip (Variables|FSM|GetCurrent_WeaponEquip)
          (:NewEnumerator0
            (if (not (Animation|CurrentMontageCheck "/Game/Animations/Montage/KATANA/Movement/AM_KatanaRolling.AM_KatanaRolling"))
              (CallFunction|PlayRolling)))))))
  (:Completed
    (switch Utilities|FlowControl|Switch|SwitchonE_WeaponType (Variables|FSM|GetCurrent_WeaponType)
      (:NewEnumerator0
        (switch Utilities|FlowControl|Switch|SwitchonE_WeaponEquip (Variables|FSM|GetCurrent_WeaponEquip)))
      (:NewEnumerator1
        (switch Utilities|FlowControl|Switch|SwitchonE_WeaponEquip (Variables|FSM|GetCurrent_WeaponEquip))))))

(event Custom|Ing_WeaponChangeKatana
  (FSM|SetWeaponType "NewEnumerator1" true)
  (FSM|SetMovement "NewEnumerator0" true)
  (Variables|이동|SetChangeWeaponEquipCompleted false))

(event Custom|Ing_WeaponChangeDagger
  (FSM|SetWeaponType "NewEnumerator0" true)
  (FSM|SetMovement "NewEnumerator0" true)
  (Variables|이동|SetChangeWeaponEquipCompleted false))

(event Input|EnhancedActionEvents|EnhancedInputActionIA_WeaponChange1
  (params (ActionValue :type Boolean) (ElapsedSeconds :type Float%20%28double-precision%29) (TriggeredSeconds :type Float%20%28double-precision%29) (InputAction :type Input%20Action%20Object%20Reference :default "/Game/InputSystem/IA_WeaponChange1.IA_WeaponChange1"))
  (:Started
    (if (Utilities|Enum|Equal(Enum) (Variables|FSM|GetCurrent_WeaponEquip) "NewEnumerator0")
      (FSM|SetWeaponEquip "NewEnumerator1" false)
      (Variables|이동|SetChangeWeaponEquipCompleted true)
      (else
        (FSM|SetWeaponType "NewEnumerator0" true)
        (FSM|SetMovement "NewEnumerator0" true)
        (Variables|이동|SetChangeWeaponEquipCompleted false)))))

(event Input|EnhancedActionEvents|EnhancedInputActionIA_WeaponChange2
  (params (ActionValue :type Boolean) (ElapsedSeconds :type Float%20%28double-precision%29) (TriggeredSeconds :type Float%20%28double-precision%29) (InputAction :type Input%20Action%20Object%20Reference :default "/Game/InputSystem/IA_WeaponChange2.IA_WeaponChange2"))
  (:Started
    (if (Utilities|Enum|Equal(Enum) (Variables|FSM|GetCurrent_WeaponEquip) "NewEnumerator0")
      (FSM|SetWeaponEquip "NewEnumerator1" false)
      (Variables|이동|SetChangeWeaponEquipCompleted true)
      (else
        (FSM|SetWeaponType "NewEnumerator1" true)
        (FSM|SetMovement "NewEnumerator0" true)
        (Variables|이동|SetChangeWeaponEquipCompleted false)))))

(event Custom|OnLandingCall_InBP)

(event EventBeginPlay
  (EventDispatchers|BindEventtoOnLandingCall (delegate Custom|OnLandingCall_InBP)))

(event EventOnMovementModeChanged
  (params (PrevMovementMode :type EMovementMode%20Enum :default "MOVE_None") (NewMovementMode :type EMovementMode%20Enum :default "MOVE_None") (PrevCustomMode :type Byte :default 0) (NewCustomMode :type Byte :default 0))
  (switch Utilities|FlowControl|Switch|SwitchonEMovementMode NewMovementMode
    (:MOVE_Falling
      (if (>= (Movement|CharacterLanding) 1e+02)
        (Movement|Jumping true)))))

(event Custom|ResetInputSacle
  (switch Utilities|FlowControl|Switch|SwitchonE_WeaponEquip (Variables|FSM|GetCurrent_WeaponEquip)
    (:NewEnumerator1
      (Variables|Movement|SetInputScale ""))
    (:NewEnumerator0
      (bind _timer (Timeline|ResetInputScleTimeline PlayFromStart)
        (:Update
          (Variables|Movement|SetInputScale (Math|Vector2D|MakeVector2D (Math|Float|Lerp (.x (Variables|Movement|GetInputScale)) 0.0 _timer) (Math|Float|Lerp (.y (Variables|Movement|GetInputScale)) 0.0 _timer))))))))

(event Custom|AttackEnd
  (Variables|Default|SetCurrentCombo 0)
  (Variables|Default|SetNextAttackCheck false)
  (Variables|Default|SetAttacking false))

(event Custom|ResetGravity
  (bind _sacle (Timeline|타임라인 PlayFromStart)
    (:Update
      (Variables|/Script/Engine.CharacterMovementComponent|SetGravityScale (Variables|Character|GetCharacterMovement) _sacle))))

(event Custom|ResetSliding
  (Variables|Movement|SetCanRolling false))

(event Custom|WeaponEquip
  (switch Utilities|FlowControl|Switch|SwitchonE_WeaponType (Variables|FSM|GetCurrent_WeaponType)
    (:NewEnumerator0
      (switch Utilities|FlowControl|Switch|SwitchonE_WeaponEquip (Variables|FSM|GetCurrent_WeaponEquip)
        (:NewEnumerator1
          (Transformation|AttachComponentToComponent (Variables|Default|GetSM_Dagger_R) (Variables|Character|GetMesh) "BP_DAGGER_R" "KeepRelative" "KeepRelative" "KeepRelative" true)
          (Transformation|AttachComponentToComponent (Variables|Default|GetSM_Dagger_L) (Variables|Character|GetMesh) "BP_DAGGER_L" "KeepRelative" "KeepRelative" "KeepRelative" true))
        (:NewEnumerator0
          (Transformation|AttachComponentToComponent (Variables|Default|GetSM_Dagger_R) (Variables|Character|GetMesh) "WEAPON_DAGGER_R" "KeepRelative" "KeepRelative" "KeepRelative" true)
          (Transformation|AttachComponentToComponent (Variables|Default|GetSM_Dagger_L) (Variables|Character|GetMesh) "WEAPON_DAGGER_L" "KeepRelative" "KeepRelative" "KeepRelative" true))))
    (:NewEnumerator1
      (switch Utilities|FlowControl|Switch|SwitchonE_WeaponEquip (Variables|FSM|GetCurrent_WeaponEquip)
        (:NewEnumerator1
          (Transformation|AttachComponentToComponent (Variables|Default|GetSK_Katana_R) (Variables|Character|GetMesh) "BP_KATANA_R" "KeepRelative" "KeepRelative" "KeepRelative" true)
          (Transformation|AttachComponentToComponent (Variables|Default|GetSK_Katana_L) (Variables|Character|GetMesh) "BP_KATANA_L" "KeepRelative" "KeepRelative" "KeepRelative" true))
        (:NewEnumerator0
          (Transformation|AttachComponentToComponent (Variables|Default|GetSK_Katana_R) (Variables|Character|GetMesh) "WEAPON_KATANA_R" "KeepRelative" "KeepRelative" "KeepRelative" true)
          (Transformation|AttachComponentToComponent (Variables|Default|GetSK_Katana_L) (Variables|Character|GetMesh) "WEAPON_KATANA_L" "KeepRelative" "KeepRelative" "KeepRelative" true))))))

(event Custom|Play_Rolling
  (bind _inputscale (Variables|Movement|GetInputScale))
  (bind _inputscale_2 (Variables|Movement|GetInputScale))
  (if (and (not (Animation|CurrentMontageCheck "/Game/Animations/Montage/DAGGER/Movement/AM_DaggerRolling.AM_DaggerRolling")) (not (Animation|CurrentMontageCheck "/Game/Animations/Montage/KATANA/Movement/AM_KatanaRolling.AM_KatanaRolling")))
    (switch Utilities|FlowControl|Switch|SwitchonE_WeaponType (Variables|FSM|GetCurrent_WeaponType)
      (:NewEnumerator0
        (if (> (.x _inputscale) 0.0)
          (Animation|Montage|PlayMontage (Variables|Character|GetMesh) "/Game/Animations/Montage/DAGGER/Movement/AM_DaggerRolling.AM_DaggerRolling" 1.0 0.0 "R")
          (elif (< (.x _inputscale) 0.0)
            (Animation|Montage|PlayMontage (Variables|Character|GetMesh) "/Game/Animations/Montage/DAGGER/Movement/AM_DaggerRolling.AM_DaggerRolling" 1.0 0.0 "L")
            (elif (< (.y _inputscale) 0.0)
              (Animation|Montage|PlayMontage (Variables|Character|GetMesh) "/Game/Animations/Montage/DAGGER/Movement/AM_DaggerRolling.AM_DaggerRolling" 1.0 0.0 "B")
              (else
                (Animation|Montage|PlayMontage (Variables|Character|GetMesh) "/Game/Animations/Montage/DAGGER/Movement/AM_DaggerRolling.AM_DaggerRolling" 1.0 0.0 "F"))))))
      (:NewEnumerator1
        (if (> (.x _inputscale_2) 0.0)
          (Animation|Montage|PlayMontage (Variables|Character|GetMesh) "/Game/Animations/Montage/KATANA/Movement/AM_KatanaRolling.AM_KatanaRolling" 1.0 0.0 "R")
          (elif (< (.x _inputscale_2) 0.0)
            (Animation|Montage|PlayMontage (Variables|Character|GetMesh) "/Game/Animations/Montage/KATANA/Movement/AM_KatanaRolling.AM_KatanaRolling" 1.0 0.0 "L")
            (elif (< (.y _inputscale_2) 0.0)
              (Animation|Montage|PlayMontage (Variables|Character|GetMesh) "/Game/Animations/Montage/KATANA/Movement/AM_KatanaRolling.AM_KatanaRolling" 1.0 0.0 "B")
              (else
                (Animation|Montage|PlayMontage (Variables|Character|GetMesh) "/Game/Animations/Montage/KATANA/Movement/AM_KatanaRolling.AM_KatanaRolling" 1.0 0.0 "F")))))))))

(event Custom|Play_Sliding
  (bind _currentmontage (Animation|GetCurrentAnimMontage))
  (bind _inputscale (Variables|Movement|GetInputScale))
  (if (and (!= _currentmontage "/Game/Animations/Montage/DAGGER/Movement/AM_DaggerSlide.AM_DaggerSlide") (!= "/Game/Animations/Montage/DAGGER/Movement/AM_DaggerRolling.AM_DaggerRolling" _currentmontage))
    (if (> (.x _inputscale) 0.0)
      (Animation|Montage|PlayMontage (Variables|Character|GetMesh) "/Game/Animations/Montage/DAGGER/Movement/AM_DaggerSlide.AM_DaggerSlide" 1.0 0.0 "R")
      (elif (< (.x _inputscale) 0.0)
        (Animation|Montage|PlayMontage (Variables|Character|GetMesh) "/Game/Animations/Montage/DAGGER/Movement/AM_DaggerSlide.AM_DaggerSlide" 1.0 0.0 "L")
        (elif (< (.y _inputscale) 0.0)
          (Animation|Montage|PlayMontage (Variables|Character|GetMesh) "/Game/Animations/Montage/DAGGER/Movement/AM_DaggerSlide.AM_DaggerSlide" 1.0 0.0 "B")
          (else
            (Animation|Montage|PlayMontage (Variables|Character|GetMesh) "/Game/Animations/Montage/DAGGER/Movement/AM_DaggerSlide.AM_DaggerSlide" 1.0 0.0 "F")))))))

(event EventSetPosition
  (params (Position :type Vector :default "0, 0, 0"))
  (Variables|이동|SetSavePosition Position))

(fn GetPosition
  (return (Variables|이동|GetSavePosition)))
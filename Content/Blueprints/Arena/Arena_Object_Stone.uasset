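; Arena stone prop whose three winter rock meshes can fade their snow effect in and out.
; BeginPlay sets the "Snow Bias" material scalar on all three meshes to a low starting value.
; PlaySnow plays a timeline that writes its Alpha into that parameter on each update, and EndSnow reverses the same timeline.
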(event EventBeginPlay
  (Rendering|Material|SetScalarParameterValueonMaterials (Variables|Default|GetSM_WinterRock_D) "Snow Bias" -3.0))

(event Collision|EventActorBeginOverlap
  (params (OtherActor :type Actor%20Object%20Reference)))

(event EventTick
  (params (DeltaSeconds :type Float%20%28single-precision%29)))

(event EventPlaySnow
  (bind _alpha (Timeline|TL_SnowPlay Play)
    (:Update
      (Rendering|Material|SetScalarParameterValueonMaterials (Variables|Default|GetSM_WinterRock_D) "Snow Bias" _alpha))))

(event EventEndSnow
  (bind _alpha (Timeline|TL_SnowPlay Reverse)
    (:Update
      (Rendering|Material|SetScalarParameterValueonMaterials (Variables|Default|GetSM_WinterRock_D) "Snow Bias" _alpha))))

(fn ConstructionScript)
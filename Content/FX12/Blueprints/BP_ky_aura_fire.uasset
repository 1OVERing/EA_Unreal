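; BP_ky_aura_fire is a fire aura effect actor that damages what is around it.
; While its FX is active, each tick runs a multi-sphere trace at its location and applies fire-typed damage to hit actors.
; Hit actors join the trace's ignore list, which is never cleared here, so later ticks skip them.
; BeginPlay enables timed debug drawing from the game instance's attack-trace option.
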(event EventBeginPlay
  (|CallParentFunction)
  (bind _asbp_game_instance (Utilities|Casting|CastToBP_GameInstance (Game|GetGameInstance)))
  (if (.onattackdebugtrace (Variables|/Game/Blueprints/Systems/BP_GameInstance.BP_GameInstance_C|GetGameOption _asbp_game_instance))
    (Variables|Default|SetDrawType "ForDuration")
    (else
      (Variables|Default|SetDrawType "None"))))

(event Collision|EventActorBeginOverlap
  (params (OtherActor :type Actor%20Object%20Reference))
  (|CallParentFunction OtherActor) ; This node is disabled and will not be called.\nDrag off pins to build functionality.
)

(event EventTick
  (params (DeltaSeconds :type Float%20%28single-precision%29))
  (bind _returnvalue (Transformation|GetActorLocation))
  (|CallParentFunction DeltaSeconds)
  (if (Components|Activation|IsActive (Variables|Default|GetFX))
    (bind (_outhits _returnvalue_2) (Collision|MultiSphereTraceByChannel _returnvalue _returnvalue 5e+02 "TraceTypeQuery4" false (Variables|Default|GetActors) (Variables|Default|GetDrawType)))
    (if _returnvalue_2
      (for _array_element _outhits
        (Utilities|Array|AddUnique (Variables|Default|GetActors) (.HitActor (Collision|BreakHitResult _array_element)))
        (Game|Damage|ApplyDamage (.HitActor (Collision|BreakHitResult _array_element)) 1.0 0 0 "/Game/Blueprints/DTBP/DTBP_Fire.DTBP_Fire_C")))))

(fn ConstructionScript
  (|CallParentFunction))